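; BP_Enemy is a melee enemy character that wanders around its spawn point and chases and punches the player when within range.
; Tick updates the range flag, while AggroState loops between Wander and ChasePlayer through AIMoveTo results.
; A montage notify triggers a sphere trace that applies punch damage.
; Taking damage knocks it back or, at zero health, ragdolls it; the spawn-distance check has no effect yet.
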(event Custom|Wander
  ;[0.125 0.125 0.125] Wander
  (AI|AIMoveTo self (.RandomLocation (AI|Navigation|GetRandomReachablePointinRadius (Variables|Default|GetSpawnPoint) 6e+02 0 0)) 0 5.0 false
    (:OnSuccess
      (if (Variables|Default|GetInRangeOfPlayer)
        _
        (else
          (Utilities|FlowControl|Delay (Math|Random|RandomFloatinRange 1.0 3.0)))))
    (:OnFail
      _))
  (CallFunction|AggroState))

(event Custom|ActivatePunchCollider
  (bind _attack_trace_pas_enemy (Variables|Default|GetAttack%20Trace%20Pas%20Enemy))
  (bind _returnvalue (Transformation|GetWorldLocation _attack_trace_pas_enemy))
  ;[0.125 0.125 0.125] Activate Punch Collider
  (bind (_outhit _returnvalue_2) (Collision|SphereTraceForObjects _returnvalue (+ _returnvalue (* (Math|Vector|GetForwardVector _attack_trace_pas_enemy) 35.0)) 25.0 (Utilities|Array|MakeArray "ObjectTypeQuery3") false 0 "ForDuration"))
  (if _returnvalue_2
    (Game|Damage|ApplyDamage (.HitActor (Collision|BreakHitResult _outhit)) 1e+01 0 0)))

(event Custom|Punch
  ;[0.125 0.125 0.125] Punch
  (if (Variables|Default|GetCanPunchEnemy)
    (Animation|Montage|PlayMontage (Variables|Character|GetMesh) "/Game/Punch_Sequence_Montage.Punch_Sequence_Montage"
      (:then
        (Variables|Default|SetCanPunchEnemy false))
      (:OnCompleted
        (Variables|Default|SetCanPunchEnemy true))
      (:OnNotifyBegin
        (CallFunction|ActivatePunchCollider)))))

(event Custom|AggroState
  ;[0.125 0.125 0.125] Aggro State
  (if (Variables|Default|GetAlive)
    (if (Variables|Default|GetInRangeOfPlayer)
      (CallFunction|ChasePlayer)
      (else
        (CallFunction|Wander)))))

(event Custom|CheckPlayerDistance
  ;[0.125 0.125 0.125] Check Player Distance
  (if (<= 8e+02 (Transformation|GetDistanceTo (Game|GetPlayerCharacter 0)))
    (Variables|Default|SetInRangeOfPlayer false)
    (else
      (Variables|Default|SetInRangeOfPlayer true))))

(event Custom|CheckSpawnDistance
  ;[0.125 0.125 0.125] Check Spawn Distance
  (if (<= 1e+03 (Math|Vector|Distance(Vector) (Transformation|GetActorLocation) (Variables|Default|GetSpawnPoint)))
    _))

(event Custom|ChasePlayer
  ;[0.125 0.125 0.125] Chase Player
  (if (Variables|Default|GetAlive)
    (AI|AIMoveTo self "0, 0, 0" (Game|GetPlayerCharacter 0) 5.0 false
      (:OnSuccess
        (Utilities|FlowControl|Delay 0.5)
        (CallFunction|Punch))
      (:OnFail
        _))
    (CallFunction|AggroState)))

(event EventTick
  (params (DeltaSeconds :type Float%20%28single-precision%29))
  ;[0.125 0.125 0.125] Tick
  (CallFunction|CheckSpawnDistance)
  (CallFunction|CheckPlayerDistance))

(event Game|Damage|EventAnyDamage
  (params (Damage :type Float%20%28single-precision%29) (DamageType :type Damage%20Type%20Object%20Reference) (InstigatedBy :type Controller%20Object%20Reference) (DamageCauser :type Actor%20Object%20Reference))
  ;[0.125 0.125 0.125] Take Damage
  (bind _output_get (Variables|Default|SetHealth (- (Variables|Default|GetHealth) Damage)))
  (if (<= _output_get 0.0)
    (Variables|Default|SetAlive false)
    (Physics|SetSimulatePhysics (Variables|Character|GetMesh) true)
    (Components|DestroyComponent (Variables|Collision|GetCapsuleComponent))
    (else
      (Character|LaunchCharacter (+ (* (Transformation|GetActorForwardVector) -2e+02) (* (Transformation|GetActorUpVector) 1e+02)) false false))))

(event EventBeginPlay
  ;[0.125 0.125 0.125] BeginPlay
  (Variables|Default|SetSpawnPoint (Transformation|GetActorLocation))
  (CallFunction|AggroState))

(fn ConstructionScript)